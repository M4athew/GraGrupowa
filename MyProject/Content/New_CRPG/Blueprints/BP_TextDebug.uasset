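; BP_TextDebug is an actor with a TextRender and a Box trigger, named as a debug text helper.
; Three boolean flags gate visibility changes at BeginPlay, overlap begin and overlap end.
; All three paths hide the text, including the AlwaysShowText one, and none shows it.
; Any overlapping actor triggers the logic, since the casts to BP_CRPG_PlayerCharacter are unconnected.
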(event `self.ReceiveBeginPlay`
  (`parent.ReceiveBeginPlay`)
  (if (`self.AlwaysShowText`)
    (`SceneComponent.SetVisibility` (`self.TextRender`) false false)))

(event `self.Box.OnComponentBeginOverlap`
  (params (OverlappedComponent :type "PrimitiveComponent Object Reference") (OtherActor :type "Actor Object Reference") (OtherComp :type "PrimitiveComponent Object Reference") (OtherBodyIndex :type Integer) (bFromSweep :type Boolean) (SweepResult :type "HitResult Structure (by ref)"))
  (if (`self.UseTextRender?`)
    (`SceneComponent.SetVisibility` (`self.TextRender`) false false)))

(event `self.Box.OnComponentEndOverlap`
  (params (OverlappedComponent :type "PrimitiveComponent Object Reference") (OtherActor :type "Actor Object Reference") (OtherComp :type "PrimitiveComponent Object Reference") (OtherBodyIndex :type Integer))
  (if (`self.DeactivateWhen Left?`)
    (`SceneComponent.SetVisibility` (`self.TextRender`) false false)))

(fn `UserConstructionScript`
  (`parent.UserConstructionScript`))