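; BP_FunctionLibrary is a function library of shortcuts to the CRPG project's core gameplay objects.
; It returns player 0's character and the game state, each cast to its project class.
; The HUD getter reads MainHUDRef from the game state, so that reference is held there.
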(fn `GetProjecHUD`
  (returns (MainHUDRef :type "UserWidget Object Reference"))
  (return (`/Game/New_CRPG/Blueprints/BP_CRPG_GameState.MainHUDRef` (`self.GetProjectGameState` null))))

(fn `GetProjectGameState`
  (returns (`AsBP CRPG Game State` :type "/Game/New_CRPG/Blueprints/BP_CRPG_GameState Object Reference"))
  (bind _asbp_crpg_game_state (cast `/Game/New_CRPG/Blueprints/BP_CRPG_GameState` (`GameplayStatics.GetGameState` null)))
  (return _asbp_crpg_game_state))

(fn `GetProjectPlayer`
  (returns (Player :type "/Game/New_CRPG/Blueprints/Player/BP_CRPG_PlayerCharacter Object Reference"))
  (bind _asbp_crpg_player_character (cast `/Game/New_CRPG/Blueprints/Player/BP_CRPG_PlayerCharacter` (`GameplayStatics.GetPlayerCharacter` null)))
  (return _asbp_crpg_player_character))